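; BP_HunterCharacter is a third-person combat character that adds touch controls, hit feedback and a switchable over-the-shoulder camera.
; Touch thumbstick and button events forward to move, look, combo attack and charged attack functions defined outside these graphs.
; Dealing damage triggers a camera shake at the impact point, while receiving it adds a directional Niagara effect and its own shake.
; A FlipFlop-driven timeline smoothly swaps the camera boom's shoulder offset, which the construction script initializes.
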(event EventTouchComboAttackStart
  ;[0.15 0.15 0.15 0.5] Touch input for Third Person Combat
  (Class|CombatCharacter|DoComboAttackStart))

(event EventToggleCamera
  ;[0.15 0.15 0.15 0.5] Camera
  ;;[0.15 0.15 0.15 0.5] Use a timeline to smoothly toggle between normal and negative shoulder offsets.
  (Utilities|FlowControl|FlipFlop
    (:A
      (bind _side (Timeline|Timeline Play)
        (:Update
          ;;[0.15 0.15 0.15 0.5] Update the third person camera offset
          (Transformation|SetRelativeLocation (Variables|Default|GetCameraBoom) (Math|Vector|MakeVector 0.0 (* _side (Variables|Camera|GetShoulder%20Offset)) (Variables|Camera|GetCamera%20Height)) false false))))
    (:B
      (Timeline|Timeline Reverse))))

(event EventPrimaryThumbstick
  (params (Axis :type Vector%202D%20Structure))
  ;[0.15 0.15 0.15 0.5] Touch input for Third Person Combat
  (Class|CombatCharacter|DoMove (.x Axis) (.y Axis)))

(event EventSecondaryThumbstick
  (params (Axis :type Vector%202D%20Structure))
  ;[0.15 0.15 0.15 0.5] Touch input for Third Person Combat
  (Class|CombatCharacter|DoLook (.x Axis) (.y Axis)))

(event EventTouchComboAttackEnd
  ;[0.15 0.15 0.15 0.5] Touch input for Third Person Combat
  (Class|CombatCharacter|DoComboAttackEnd))

(event EventDealtDamage
  (params (Damage :type Float%20%28single-precision%29) (ImpactPoint :type Vector%20%28by%20ref%29 :default "0, 0, 0"))
  ;[0.15 0.15 0.15 0.5] Play effects when dealing and receiving damage
  (Camera|PlayWorldCameraShake "/Game/Variant_Combat/Blueprints/BP_CameraShake_Hit_Enemy.BP_CameraShake_Hit_Enemy_C" ImpactPoint 0.0 5e+02))

(event EventdDamage
  (params (Damage :type Float%20%28single-precision%29) (ImpactPoint :type Vector%20%28by%20ref%29 :default "0, 0, 0") (DamageDirection :type Vector%20%28by%20ref%29 :default "0, 0, 0"))
  ;[0.15 0.15 0.15 0.5] Play effects when dealing and receiving damage
  (Niagara|SpawnSystematLocation "/Game/Variant_Combat/VFX/NS_Damage.NS_Damage" ImpactPoint (Math|Conversions|RotationFromXVector DamageDirection))
  (Camera|PlayWorldCameraShake "/Game/Variant_Combat/Blueprints/BP_CameraShake_Hit_Player.BP_CameraShake_Hit_Player_C" ImpactPoint 0.0 5e+02))

(event EventTouchChargedAttackStart
  ;[0.15 0.15 0.15 0.5] Touch input for Third Person Combat
  (Class|CombatCharacter|DoChargedAttackStart))

(event EventTouchChargedAttackEnd
  ;[0.15 0.15 0.15 0.5] Touch input for Third Person Combat
  (Class|CombatCharacter|DoChargedAttackEnd))

(event EventTouchToggleCamera
  ;[0.15 0.15 0.15 0.5] Camera
  ;;[0.15 0.15 0.15 0.5] Use a timeline to smoothly toggle between normal and negative shoulder offsets.
  (Utilities|FlowControl|FlipFlop
    (:A
      (bind _side (Timeline|Timeline Play)
        (:Update
          ;;[0.15 0.15 0.15 0.5] Update the third person camera offset
          (Transformation|SetRelativeLocation (Variables|Default|GetCameraBoom) (Math|Vector|MakeVector 0.0 (* _side (Variables|Camera|GetShoulder%20Offset)) (Variables|Camera|GetCamera%20Height)) false false))))
    (:B
      (Timeline|Timeline Reverse))))

(fn ConstructionScript
  ;[0.15 0.15 0.15 0.5] Set the third person camera offset.
  (Transformation|SetRelativeLocation (Variables|Default|GetCameraBoom) (Math|Vector|MakeVector 0.0 (Variables|Camera|GetShoulder%20Offset) (Variables|Camera|GetCamera%20Height)) false false))